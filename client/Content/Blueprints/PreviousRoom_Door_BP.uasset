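; PreviousRoom_Door_BP is a door that sends the game back to the previous room's level when it registers a Hit event.
; It reads the current level name and runs a chain of name comparisons that opens a hard-coded predecessor level, leading back through the house rooms toward ThirdPersonMap.
; A Library-to-LivingRoom branch exists but is disconnected, so the door does nothing in that level.
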(event `self.ReceiveActorBeginOverlap`
  (params (OtherActor :type "Actor Object Reference")))

(event `self.ReceiveHit`
  (params (MyComp :type "PrimitiveComponent Object Reference") (Other :type "Actor Object Reference") (OtherComp :type "PrimitiveComponent Object Reference") (bSelfMoved :type Boolean) (HitLocation :type "Vector Structure") (HitNormal :type "Vector Structure") (NormalImpulse :type "Vector Structure") (Hit :type "HitResult Structure (by ref)"))
  (bind _returnvalue (`GameplayStatics.GetCurrentLevelName` true))
  (bind _output_get (set `self.CurrnetLevel` _returnvalue))
  (if (`KismetStringLibrary.EqualEqual_StrStr` _output_get "LivingRoom")
    (`GameplayStatics.OpenLevel` "ThirdPersonMap")
    (elif (`KismetStringLibrary.EqualEqual_StrStr` _output_get "DiningRoom")
      (`GameplayStatics.OpenLevel` "LivingRoom")
      (elif (`KismetStringLibrary.EqualEqual_StrStr` _output_get "Kitchen")
        (`GameplayStatics.OpenLevel` "DiningRoom")
        (elif (`KismetStringLibrary.EqualEqual_StrStr` _output_get "BedRoom")
          (`GameplayStatics.OpenLevel` "LivingRoom")
          (elif (`KismetStringLibrary.EqualEqual_StrStr` _output_get "BathRoom")
            (`GameplayStatics.OpenLevel` "BedRoom")))))))

(fn `UserConstructionScript`)
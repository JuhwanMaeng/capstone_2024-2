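; Planner actor that sets NPC destinations from a remote time-based schedule service.
; Tick watches the seconds digits of GameInstance WorldTime, using a DoOnce and busy flag to fire one HTTP POST of the time at each "00".
; It slices the response by substring search into Ethan, Jack and Lily destinations on the GameInstance.
; It then sends NewDestinationMessage to the Dialogue_BPI actors cached at BeginPlay.
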(event `self.ReceiveBeginPlay`
  (bind _asmy_game_instance_bp (cast `/Game/Blueprints/myGameInstance_BP` (`GameplayStatics.GetGameInstance`)))
  (set `self.GameInstance_REF` _asmy_game_instance_bp)
  (bind _outactors (`GameplayStatics.GetAllActorsWithInterface` "/Game/Tiles/NPC/Dialogue_BPI.Dialogue_BPI_C"))
  (set `self.NPC_Array` _outactors))

(event `self.ReceiveTick`
  (params (DeltaSeconds :type "Float (single-precision)"))
  (bind _timeresponse (`self.timeResponse`))
  (bind _timeresponse_2 (`self.timeResponse`))
  (bind _timeresponse_3 (`self.timeResponse`))
  (bind _returnvalue (`KismetTextLibrary.Conv_TextToString` (`/Game/Blueprints/myGameInstance_BP.worldTime` (`self.GameInstance_REF`))))
  (bind _returnvalue_2 (+ (`KismetStringLibrary.FindSubstring` _timeresponse "Lily") 7))
  (bind _returnvalue_3 (+ (`KismetStringLibrary.FindSubstring` _timeresponse_2 "Ethan") 8))
  (bind _returnvalue_4 (+ (`KismetStringLibrary.FindSubstring` _timeresponse_3 "Jack") 7))
  (bind _returnvalue_5 (`KismetStringLibrary.GetSubstring` _returnvalue 17 2))
  (if (`KismetStringLibrary.NotEqual_StrStr` _returnvalue_5 "00")
    (goto _label :!via `Reset`)
    (elif (and (not (`self.branchbool`)) (`KismetStringLibrary.EqualEqual_StrStr` "00" _returnvalue_5))
      (`/Engine/EditorBlueprintResources/StandardMacros.DoOnce` false :!label _label
        (:`Completed`
          (set `self.branchbool` true)
          (bind (_outheader _result_body) (`|HttpRequest` "http://awaiapi.eastus.cloudapp.azure.com:7000/time" "Post" (`|MakeRequestHeader` "Json") (`KismetStringLibrary.Concat_StrStr` "{\"time\" : \"" _returnvalue "\"}"))
            (:`On Success`
              (set `self.timeResponse` _result_body)
              (set `/Game/Blueprints/myGameInstance_BP.Ethan_Destination` (`KismetStringLibrary.GetSubstring` _timeresponse_2 _returnvalue_3 (- (- (`KismetStringLibrary.FindSubstring` _timeresponse_2 "Jack") 5) _returnvalue_3)) (`self.GameInstance_REF`))
              (set `/Game/Blueprints/myGameInstance_BP.Jack_Destination` (`KismetStringLibrary.GetSubstring` _timeresponse_3 _returnvalue_4 (- (- (`KismetStringLibrary.FindSubstring` _timeresponse_3 "Lily") 5) _returnvalue_4)) (`self.GameInstance_REF`))
              (set `/Game/Blueprints/myGameInstance_BP.Lily_Destination` (`KismetStringLibrary.GetSubstring` _timeresponse _returnvalue_2 (- (- (`KismetStringLibrary.FindSubstring` _timeresponse "}]") 1) _returnvalue_2)) (`self.GameInstance_REF`))
              (message `/Game/Tiles/NPC/Dialogue_BPI.New_Destination` (`self.NPC_Array`))
              (set `self.branchbool` false))))))))

(fn `UserConstructionScript`)
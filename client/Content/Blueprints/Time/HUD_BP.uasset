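; HUD Blueprint that puts the room number, world time and chat widgets on screen.
; BeginPlay caches the custom game instance, then creates the room number and world time widgets and adds them to the viewport.
; Tick polls the game instance's IsChatting flag and, after a one-second Delay, adds a new chat widget, repeating while the flag stays true without removing earlier ones.
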(event `self.ReceiveBeginPlay`
  (bind _asmy_game_instance_bp (cast `/Game/Blueprints/myGameInstance_BP` (`GameplayStatics.GetGameInstance`)))
  (set `self.As My Game Instance BP` _asmy_game_instance_bp)
  (bind _returnvalue (`|CreateWidget` "/Game/Blueprints/Time/RoomNum_WB.RoomNum_WB_C"))
  (bind _output_get (set `self.RoomNum_REF` _returnvalue))
  (`UserWidget.AddToViewport` _output_get 0)
  (bind _returnvalue_2 (`|CreateWidget` "/Game/Blueprints/Time/WorldTime_WB.WorldTime_WB_C"))
  (bind _output_get_2 (set `self.Worldtime_REF` _returnvalue_2))
  (`UserWidget.AddToViewport` _output_get_2 0))

(event `self.ReceiveTick`
  (params (DeltaSeconds :type "Float (single-precision)"))
  (if (`/Game/Blueprints/myGameInstance_BP.isChatting` (`self.As My Game Instance BP`))
    (`KismetSystemLibrary.Delay` 1.0)
    (bind _returnvalue (`|CreateWidget` "/Game/Blueprints/Chat_WB.Chat_WB_C"))
    (bind _output_get (set `self.Chat_REF` _returnvalue))
    (`UserWidget.AddToViewport` _output_get 0)))

(fn `UserConstructionScript`)
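; Timetable actor that drives timed NPC conversations from a remote HTTP server.
; Tick, gated by CanEnter, fetches the current plot, retrying after a delay on failure, then requests its info into PlanList.
; A delayed loop polls the chat endpoint, slicing time, speaker and line from raw JSON by substring into the game instance.
; Worldtime matching End resets the plot, but no connected node updates Worldtime.
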(event `self.ReceiveBeginPlay`
  (bind _asmy_game_instance_bp (cast `/Game/Blueprints/myGameInstance_BP` (`GameplayStatics.GetGameInstance`)))
  (set `self.Game Instance REF` _asmy_game_instance_bp))

(event `self.ReceiveTick`
  (params (DeltaSeconds :type "Float (single-precision)"))
  (bind _game_instance_ref (`self.Game Instance REF`))
  (bind _current_plot (`self.current_plot`))
  (bind _returnvalue (+ (`KismetStringLibrary.FindSubstring` _current_plot ":") 2))
  (if (`self.can_enter`)
    (if (`KismetStringLibrary.EqualEqual_StrStr` (`self.current_plot`))
      (bind (_outheader _result_body) (`|HttpRequest` "http://129.80.153.177:5000/get_plot" "Get" (`|MakeRequestHeader` "Json"))
        (:`On Success`
          (set `self.current_plot` _result_body))
        (:`On Error`
          (set `self.can_enter` false)
          (`KismetSystemLibrary.Delay` 10.0)
          (set `self.can_enter` true)))
      (else
        (set `self.can_enter` false)
        (set `self.plot` (`KismetStringLibrary.GetSubstring` _current_plot _returnvalue (- (- (`KismetStringLibrary.FindSubstring` _current_plot "}") 1) _returnvalue)))
        (bind (_outheader_2 _result_body_2) (`|HttpRequest` "http://129.80.153.177:5000/plot_info" "Post" (`|MakeRequestHeader` "Json") (`KismetStringLibrary.Concat_StrStr` "{\"plot_name\" : \"" (`self.plot`) "\"}"))
          (:`On Success`
            (set `self.plan_list` _result_body_2)
            (set `/Game/Blueprints/myGameInstance_BP.isChatting` true (`self.Game Instance REF`))
            (if (`self.isnotEnd?`) :!label _label
              (bind (_outheader_3 _result_body_3) (`|HttpRequest` "http://129.80.153.177:5000/chat" "Post" (`|MakeRequestHeader` "Json") (`KismetStringLibrary.Concat_StrStr` "{\"plot_name\" : \"" (`self.plot`) "\"}"))
                (:`On Success`
                  (set `/Game/Blueprints/myGameInstance_BP.worldTime` (`KismetTextLibrary.Conv_StringToText` (`KismetStringLibrary.GetSubstring` _result_body_3 (+ (`KismetStringLibrary.FindSubstring` _result_body_3 "time") 7) 5)) _game_instance_ref)
                  (bind _returnvalue_2 (+ (`KismetStringLibrary.FindSubstring` _result_body_3 ",") 2))
                  (bind _returnvalue_3 (`KismetStringLibrary.FindSubstring` _result_body_3 ":" false true))
                  (set `/Game/Blueprints/myGameInstance_BP.chattingNPC` (`KismetStringLibrary.GetSubstring` _result_body_3 _returnvalue_2 (- (- _returnvalue_3 1) _returnvalue_2)) _game_instance_ref)
                  (bind _returnvalue_4 (+ _returnvalue_3 2))
                  (set `/Game/Blueprints/myGameInstance_BP.whatChatting` (`KismetStringLibrary.GetSubstring` _result_body_3 _returnvalue_4 (- (- (`KismetStringLibrary.FindSubstring` _result_body_3 "}" false true) 1) _returnvalue_4)) _game_instance_ref)
                  (if (`KismetTextLibrary.EqualEqual_TextText` (`self.worldtime`) (`self.end`))
                    (set `self.isnotEnd?` false)
                    (goto _label)
                    (else
                      (`KismetSystemLibrary.Delay` 5.0)
                      (goto _label)))))
              (else
                (set `self.current_plot` "None")
                (set `self.isnotEnd?` true)
                (set `/Game/Blueprints/myGameInstance_BP.isChatting` false (`self.Game Instance REF`))
                (set `self.can_enter` true)))))))))

(fn `UserConstructionScript`)
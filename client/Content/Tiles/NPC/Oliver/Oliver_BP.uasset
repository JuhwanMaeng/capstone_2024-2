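; Oliver NPC that wanders by AI moves to random nearby reachable points and can be talked to by the player.
; Talk shows the Player_Talk_WB widget; Tick halts movement while talking and resumes roaming once the game instance clears the talking flag.
; NewDestination teleports the NPC to a hardcoded spot for the location named in the game instance, then roams.
; Despite the asset's name, it uses the game instance's Ethan talking and destination variables.
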(event `Roam`
  ;[1 1 1] Roam
  (if (not (`self.stopRoaming`))
    (`|AIMoveTo` self (`NavigationSystemV1.K2_GetRandomReachablePointInRadius` (`self.K2_GetActorLocation`) 1000.0 null null) null
      (:`OnSuccess`
        _)
      (:`OnFail`
        _))
    (`self.Roam`)))

(event `self.ReceiveBeginPlay`
  ;[1 1 1] BeginPlay
  (bind _asmy_game_instance_bp (cast `/Game/Blueprints/myGameInstance_BP` (`GameplayStatics.GetGameInstance`)))
  (set `self.GameInstance_REF` _asmy_game_instance_bp)
  (`self.Roam`))

(event `self.ReceiveTick`
  (params (DeltaSeconds :type "Float (single-precision)"))
  (bind _gameinstance_ref (`self.GameInstance_REF`))
  ;[1 1 1] Tick 이벤트
  (`|ExecutionSequence`
    (:`then_0`
      (if (`self.isTalking`)
        (`MovementComponent.StopMovementImmediately` (`self.CharacterMovement`))
        (set `self.stopRoaming` true)))
    (:`then_1`
      (if (`/Game/Blueprints/myGameInstance_BP.quitTalking` (`self.GameInstance_REF`))
        (set `/Game/Blueprints/myGameInstance_BP.quitTalking` false _gameinstance_ref)
        (set `/Game/Blueprints/myGameInstance_BP.Ethan_isTalking` false _gameinstance_ref)))
    (:`then_2`
      (if (and (== (`self.isTalking`) true) (== (`/Game/Blueprints/myGameInstance_BP.Ethan_isTalking` (`self.GameInstance_REF`)) false))
        (set `self.isTalking` false)
        (set `self.stopRoaming` false)
        (`KismetSystemLibrary.Delay` 2.0)
        (`self.Roam`)))))

(event `/Game/Tiles/NPC/Dialogue_BPI.Talk`
  ;[1 1 1] Talk 이벤트
  (set `/Game/Blueprints/myGameInstance_BP.Ethan_isTalking` true (`self.GameInstance_REF`))
  (set `self.isTalking` true)
  (bind _returnvalue (`|CreateWidget` "/Game/Tiles/NPC/Player_Talk_WB.Player_Talk_WB_C" (`GameplayStatics.GetPlayerController` 0)))
  (bind _output_get (set `self.player_UI` _returnvalue))
  (`UserWidget.AddToViewport` _output_get 0))

(event `/Game/Tiles/NPC/Dialogue_BPI.New_Destination`
  ;[1 1 1] New_Destination
  (if (`self.stopRoaming`)
    _
    (elif (`KismetStringLibrary.EqualEqual_StrStr` (`/Game/Blueprints/myGameInstance_BP.Ethan_Destination` (`self.GameInstance_REF`)) "Ethan's home")
      (set `self.next_Location` (3060.0 1140.0 0.0))
      (`MovementComponent.StopMovementImmediately` (`self.CharacterMovement`) :!label _label)
      (`self.K2_TeleportTo` (`self.next_Location`) (struct :`Yaw` -90.0))
      (`self.Roam`)
      (elif (`KismetStringLibrary.EqualEqual_StrStr` (`/Game/Blueprints/myGameInstance_BP.Ethan_Destination` (`self.GameInstance_REF`)) "Mart")
        (set `self.next_Location` (2500.0 1070.0 0.0))
        (goto _label)
        (elif (`KismetStringLibrary.EqualEqual_StrStr` (`/Game/Blueprints/myGameInstance_BP.Ethan_Destination` (`self.GameInstance_REF`)) "Park")
          (set `self.next_Location` (2070.0 2720.0 0.0))
          (goto _label)
          (elif (`KismetStringLibrary.EqualEqual_StrStr` (`/Game/Blueprints/myGameInstance_BP.Ethan_Destination` (`self.GameInstance_REF`)) "Workplace")
            (set `self.next_Location` (1140.0 1410.0 0.0))
            (goto _label)
            (elif (`KismetStringLibrary.EqualEqual_StrStr` (`/Game/Blueprints/myGameInstance_BP.Ethan_Destination` (`self.GameInstance_REF`)) "School")
              (set `self.next_Location` (2950.0 2710.0 0.0))
              (goto _label))))))))

(fn `UserConstructionScript`)